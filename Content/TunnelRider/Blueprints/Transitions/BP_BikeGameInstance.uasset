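; BP_BikeGameInstance is the Tunnel Rider game instance, holding run state such as health, death, speed modifier and out-of-time status.
; Its RestartGame function resets health, interpolated health and the speed modifier to their starting values and clears the dead and out-of-time flags.
; It then sets game-only input with the mouse cursor shown, removes all widgets and reopens the start level by name.
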(fn RestartGame
  (bind _returnvalue (Game|GetPlayerController 0))
  (bind _output_get (Variables|Default|SetCurrentHealth (Variables|Default|GetMaxHealth)))
  (Variables|Default|SetInterpolatedHealth _output_get)
  (Variables|Default|SetIsDead false)
  (Variables|Default|SetCurrentSpeedModifier (Variables|Default|GetStartingSpeedModifier))
  (Variables|Default|SetIsOutOfTime false)
  (Input|SetInputModeGameOnly _returnvalue)
  (Variables|/Script/Engine.PlayerController|SetbShowMouseCursor _returnvalue true)
  (Viewport|RemoveAllWidgets)
  (Game|OpenLevel(byName) (Variables|Default|GetStartLevel)))